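; Boat race game mode that connects the player and two AI ships to race start, finish and HUD progress events.
; BeginPlay finds ships by actor tag, records start and finish marker locations, then after a short delay adds three boat markers to the HUD progress widget.
; Race events start or end the ships, while progress updates move the markers and print debug values.
; Countdown and rank-change events are empty.
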(event `self.ReceiveBeginPlay`
  (`|ExecutionSequence`
    (:`then_0`
      (`|ExecutionSequence`
        (:`then_0`
          (bind _outactors (`GameplayStatics.GetAllActorsOfClass` "/Game/LxsTestData/BP_Basic/BP_Ship.BP_Ship_C"))
          (for _array_element _outactors
            (`|ExecutionSequence`
              (:`then_0`
                (if (`self.ActorHasTag` _array_element "Player")
                  (bind _output_get (set `self.GetPlayerBoat` _array_element))
                  (set `self.PlayerBoat` _output_get)))
              (:`then_1`
                (if (`self.ActorHasTag` _array_element "AI01")
                  (set `self.GetAI01Boat` _array_element)
                  (set `self.AIBoat1` _array_element)))
              (:`then_2`
                (if (`self.ActorHasTag` _array_element "AI02")
                  (bind _output_get_2 (set `self.GetAI02Boat` _array_element))
                  (set `self.AIBoat2` _output_get_2))))))))
    (:`then_1`
      (bind _returnvalue (`GameplayStatics.GetActorOfClass` "/Game/LxsTestData/BP_Basic/BP_StartPos.BP_StartPos_C"))
      (set `self.StartLinePosition` (`self.K2_GetActorLocation` _returnvalue))
      (bind _returnvalue_2 (`GameplayStatics.GetActorOfClass` "/Game/LxsTestData/BP_Basic/BP_EndPos.BP_EndPos_C"))
      (set `self.FinishLinePosition` (`self.K2_GetActorLocation` _returnvalue_2)))
    (:`then_2`
      (`KismetSystemLibrary.Delay` 0.1)
      (bind _foundwidgets (`WidgetBlueprintLibrary.GetAllWidgetsOfClass` "/Game/UMG/WBP_HUD.WBP_HUD_C" false))
      (`|ExecutionSequence`
        (:`then_0`
          (bind _wbp_progress (`/Game/UMG/WBP_HUD.WBP_Progress` (`|GetArrayItem` _foundwidgets)))
          (bind _returnvalue_3 (`/Game/UMG/WBP_Progress.F_AddOneBoart` _wbp_progress 2))
          (set `self.BoatAI02UI` _returnvalue_3))
        (:`then_1`
          (bind _returnvalue_4 (`/Game/UMG/WBP_Progress.F_AddOneBoart` _wbp_progress 1))
          (set `self.BoatAI01UI` _returnvalue_4))
        (:`then_2`
          (bind _returnvalue_5 (`/Game/UMG/WBP_Progress.F_AddOneBoart` _wbp_progress 0))
          (set `self.PlayerBoatUI` _returnvalue_5))))))

(event `self.OnCountdownTick`
  (params (RemainingSeconds :type Integer)))

(event `self.OnRaceStarted`
  ;[1 1 1] 比赛开始
  (`/Game/LxsTestData/BP_Basic/BP_Ship.Event_StartRace` (`self.GetPlayerBoat`))
  (`/Game/LxsTestData/BP_Basic/BP_Ship.Event_StartRace` (`self.GetAI02Boat`))
  (`/Game/LxsTestData/BP_Basic/BP_Ship.Event_StartRace` (`self.GetAI01Boat`)))

(event `self.OnProgressUpdated`
  (params (BoatProgresses :type "Array of Float (single-precision) (by ref)") (BoatRanks :type "Array of Integer (by ref)"))
  ;[1 1 1] 赛程进度更新
  (`self.F_NotProgressUI` BoatProgresses BoatRanks)
  (`KismetSystemLibrary.PrintString` (`KismetSystemLibrary.GetObjectName` (`self.AIBoat2`)) true true (struct :`G` 0.66 :`B` 1.0 :`A` 1.0) 2.0 "AIboat02")
  (`KismetSystemLibrary.PrintString` (`KismetSystemLibrary.GetObjectName` (`self.AIBoat1`)) true true (struct :`G` 0.66 :`B` 1.0 :`A` 1.0) 2.0 "AIboat01"))

(event `self.OnRankChanged`
  (params (BoatIndex :type Integer) (OldRank :type Integer) (NewRank :type Integer))
  ;[1 1 1] 排名
)

(event `self.OnBoatFinished`
  (params (BoatIndex :type Integer) (FinishTime :type "Float (single-precision)") (FinalRank :type Integer))
  ;[1 1 1] 比赛冲线与结束
  (`KismetSystemLibrary.PrintString` "游戏结束" true true (struct :`R` 0.267087 :`G` 1.0 :`A` 1.0))
  (switch `int` BoatIndex
    (:`0`
      (`/Game/LxsTestData/BP_Basic/BP_Ship.Event_RaceEnd` (`self.GetPlayerBoat`)))
    (:`1`
      (`/Game/LxsTestData/BP_Basic/BP_Ship.Event_RaceEnd` (`self.GetAI01Boat`)))
    (:`2`
      (`/Game/LxsTestData/BP_Basic/BP_Ship.Event_RaceEnd` (`self.GetAI02Boat`)))))

(event `self.OnRaceFinished`
  (params (FinalRankings :type "Array of BoatFinalResult Structure (by ref)"))
  ;[1 1 1] 比赛冲线与结束
  (`/Game/LxsTestData/BP_Basic/BP_Ship.Event_RaceEnd` (`self.GetAI02Boat`))
  (`/Game/LxsTestData/BP_Basic/BP_Ship.Event_RaceEnd` (`self.GetAI01Boat`))
  (`/Game/LxsTestData/BP_Basic/BP_Ship.Event_RaceEnd` (`self.GetPlayerBoat`)))

(fn `F_NotProgressUI`
  (params (InputProgress :type "Array of Float (single-precision) (by ref)") (Array2 :type "Array of Integer"))
  (locals (ProgressCache :type "Array of Float (single-precision)") (NewLocalVar :type "Float (single-precision)"))
  (bind _output (`|GetArrayItem` (`local.ProgressCache`) 2))
  (bind _output_2 (`|GetArrayItem` (`local.ProgressCache`) 1))
  (bind _output_3 (`|GetArrayItem` (`local.ProgressCache`)))
  (set `local.ProgressCache` InputProgress)
  (`|ExecutionSequence`
    (:`then_0`
      (bind _playerboatui (`self.PlayerBoatUI`)
        (:`then`
          (`/Game/UMG/WBP_OneBoatPos.Event_SetPosByPercent` _playerboatui _output_3)
          (`KismetSystemLibrary.PrintString` (`KismetStringLibrary.Concat_StrStr` "当前进度" (`KismetStringLibrary.Conv_DoubleToString` _output_3)) true true (struct :`G` 0.66 :`B` 1.0 :`A` 1.0) 2.0 "船只进度"))
        (:`else`)))
    (:`then_1`
      (bind _boatai01ui (`self.BoatAI01UI`)
        (:`then`
          (`/Game/UMG/WBP_OneBoatPos.Event_SetPosByPercent` _boatai01ui _output_2)
          (`KismetSystemLibrary.PrintString` (`KismetStringLibrary.Concat_StrStr` "AI01进度" (`KismetStringLibrary.Conv_DoubleToString` _output_2)) true true (struct :`G` 0.66 :`B` 1.0 :`A` 1.0) 2.0 "AI01进度"))
        (:`else`)))
    (:`then_2`
      (bind _boatai02ui (`self.BoatAI02UI`)
        (:`then`
          (set `local.NewLocalVar` _output)
          (`/Game/UMG/WBP_OneBoatPos.Event_SetPosByPercent` _boatai02ui _output)
          (`self.AIBoat2`
            (:`then`
              (`KismetSystemLibrary.PrintString` (`KismetStringLibrary.Concat_StrStr` "AI02进度" (`KismetStringLibrary.Conv_DoubleToString` _output)) true true (struct :`G` 0.66 :`B` 1.0 :`A` 1.0) 2.0 "AI02进度"))
            (:`else`)))
        (:`else`)))
    (:`then_3`
      (return))))

(fn `UserConstructionScript`)