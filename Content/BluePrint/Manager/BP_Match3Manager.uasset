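; BP_Match3Manager bridges match-3 board events to the HUD and ships, turning matches into speed changes.
; It caches the HUD and tagged player and AI ships when the board initializes.
; Swap, clear and fall events drive HUD animations, with delays after clears and falls before calling AdvanceGameState.
; Morale and skill-point changes update the HUD, while speed triggers buff the player or slow both AIs; skill casting and reshuffle only print debug text.
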(event `self.OnBoardInitialized`
  (`KismetSystemLibrary.Delay` 0.1)
  (`|ExecutionSequence`
    (:`then_0`
      (bind _foundwidgets (`WidgetBlueprintLibrary.GetAllWidgetsOfClass` "/Game/UMG/WBP_HUD.WBP_HUD_C" false))
      (set `self.HUD` (`|GetArrayItem` _foundwidgets)))
    (:`then_1`
      (bind _outactors (`GameplayStatics.GetAllActorsOfClass` "/Game/LxsTestData/BP_Basic/BP_Ship.BP_Ship_C"))
      (for _array_element _outactors
        (`|ExecutionSequence`
          (:`then_0`
            (if (`self.ActorHasTag` _array_element "Player")
              (set `self.PlayerShip` _array_element)))
          (:`then_1`
            (if (`self.ActorHasTag` _array_element "AI01")
              (set `self.AIShip01` _array_element)))
          (:`then_2`
            (if (`self.ActorHasTag` _array_element "AI02")
              (set `self.AIShip02` _array_element))))))))

(event `self.ReceiveBeginPlay`)

(event `self.OnBoardReshuffle`
  (`KismetSystemLibrary.PrintString` "死锁" true true (struct :`R` 1.0 :`B` 0.228147 :`A` 1.0) 10.0))

(event `Key|One`
  (params (Key :type "Key Structure"))
  (:`Pressed`
    (`self.AdvanceGameState`)
    (`KismetSystemLibrary.PrintString` "触发")))

(event `self.OnFallAnimTriggered`
  (params (FallMoves :type "Array of FallMove Structure (by ref)"))
  (bind _hud (`self.HUD`)
    (:`then`
      (`/Game/UMG/WBP_PlotsOverlay.F_HandleFallData` (`/Game/UMG/WBP_HUD.WBP_PlotsOverlay` _hud) FallMoves)
      (`KismetSystemLibrary.Delay` 0.3)
      (`self.AdvanceGameState`))
    (:`else`)))

(event `self.OnMatchesCleared`
  (params (ClearedIndices :type "Array of Integer (by ref)") (TriggeredEffects :type "Array of SpecialEffectData Structure (by ref)"))
  (bind _hud (`self.HUD`)
    (:`then`
      (`/Game/UMG/WBP_PlotsOverlay.F_HandleClearAnimi` (`/Game/UMG/WBP_HUD.WBP_PlotsOverlay` _hud) ClearedIndices)
      (`/Game/UMG/WBP_HUD.F_HandleEffect` _hud TriggeredEffects (`GameplayStatics.ProjectWorldToScreen` (`GameplayStatics.GetPlayerController` 0) (`self.K2_GetActorLocation` (`self.PlayerShip`)) true))
      (`GameplayStatics.PlaySound2D` "/Game/Assets/WAV/正常消除01.正常消除01" 1.0 1.0 0.0 null null)
      (`KismetSystemLibrary.Delay` 0.4)
      (`self.AdvanceGameState`))
    (:`else`)))

(event `self.OnSwapAnimTriggered`
  (params (IndexA :type Integer) (IndexB :type Integer) (bIsSuccessful :type Boolean))
  (if bIsSuccessful
    (bind _hud (`self.HUD`)
      (:`then`
        (`/Game/UMG/WBP_PlotsOverlay.F_Sworp` (`/Game/UMG/WBP_HUD.WBP_PlotsOverlay` _hud) IndexA IndexB))
      (:`else`))
    (else
      (`KismetSystemLibrary.PrintString` "失败")
      (bind _hud_2 (`self.HUD`)
        (:`then`
          (bind _wbp_plotsoverlay (`/Game/UMG/WBP_HUD.WBP_PlotsOverlay` _hud_2))
          (`/Game/UMG/WBP_PlotsOverlay.F_Sworp` _wbp_plotsoverlay IndexA IndexB)
          (`KismetSystemLibrary.Delay` 0.2)
          (`/Game/UMG/WBP_PlotsOverlay.F_Sworp` _wbp_plotsoverlay IndexB IndexA))
        (:`else`)))))

(event `self.OnMoraleChanged`
  (params (NewMorale :type Integer) (InMaxMorale :type Integer) (AddedAmount :type Integer))
  (`KismetSystemLibrary.PrintString` (`KismetStringLibrary.Concat_StrStr` "士气变化" (`KismetStringLibrary.Conv_IntToString` NewMorale)))
  (bind _hud (`self.HUD`)
    (:`then`
      (`/Game/UMG/WBP_BoardAndSkill.Event_UPDataMorale` (`/Game/UMG/WBP_HUD.WBP_BoardAndSkill` _hud) NewMorale InMaxMorale))
    (:`else`)))

(event `self.OnSkillPointChanged`
  (params (NewSkillPoints :type Integer) (InMaxSkillPoints :type Integer))
  (`KismetSystemLibrary.PrintString` "技能点变化" true true (struct :`G` 1.0 :`B` 0.207158 :`A` 1.0) 10.0)
  (bind _hud (`self.HUD`)
    (:`then`
      (`/Game/UMG/WBP_BoardAndSkill.Event_UPdataSkillPoint` (`/Game/UMG/WBP_HUD.WBP_BoardAndSkill` _hud) NewSkillPoints))
    (:`else`)))

(event `self.OnPlayerSpeedUpTriggered`
  (params (TriggerCount :type Integer) (SpeedBoostAmount :type "Float (single-precision)"))
  (bind _playership (`self.PlayerShip`)
    (:`then`
      (`/Game/LxsTestData/BP_Basic/BP_Ship.Event_GetSpeedUP` _playership TriggerCount SpeedBoostAmount))
    (:`else`)))

(event `self.OnPlayerSlowDownEnemyTriggered`
  (params (TriggerCount :type Integer) (SlowDownAmount :type "Float (single-precision)"))
  ;[1 0 0.01695] 待做
  (`/Game/LxsTestData/BP_Basic/BP_Ship.Event_GetSpeedDown` (`self.AIShip01`) TriggerCount SlowDownAmount)
  (`/Game/LxsTestData/BP_Basic/BP_Ship.Event_GetSpeedDown` (`self.AIShip02`) TriggerCount SlowDownAmount))

(event `self.OnSkillCasted`
  (params (SkillType :type "ESkillType Enum" :default "EastWind") (Config :type "SkillConfig Structure (by ref)"))
  (`KismetSystemLibrary.PrintString` (`KismetStringLibrary.Concat_StrStr` "触发技能" (`|GetEnumeratorNameAsString` SkillType)) true true (struct :`R` 1.0 :`B` 0.179855 :`A` 1.0) 10.0 "触发技能调试")
  (switch `ESkillType` SkillType))

(fn `UserConstructionScript`)