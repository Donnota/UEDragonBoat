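; BP_Ship is a racing ship that moves along its arrow's forward vector via projectile movement once the race starts.
; Each speed-up pickup adds timestamps that expire after SpeedTime; the active count raises target speed above MinSpeed.
; Tick eases speed toward that target, or to zero after race end, and scales animation play rate with it.
; On BeginPlay it binds itself to its board-speed widget.
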(event `Event_StartRace`
  ;[1 1 1] 开始比赛
  (set `MovementComponent.Velocity` (* (`SceneComponent.GetForwardVector` (`self.Arrow`)) (`self.NowSpeed`)) (`self.ProjectileMovement`))
  (`SkeletalMeshComponent.SetPlayRate` (`self.SkeletalMesh1`) 1.0)
  (set `self.RaceStart` true))

(event `self.ReceiveBeginPlay`
  ;[1 1 1] 初始化
  (`SkeletalMeshComponent.SetPlayRate` (`self.SkeletalMesh1`) 0.0)
  (bind _aswbp_board_speed (cast `/Game/UMG/WBP_BoardSpeed` (`WidgetComponent.GetWidget` (`self.Widget`))))
  (bind _output_get (set `self.As WBP Board Speed` _aswbp_board_speed))
  (set `/Game/UMG/WBP_BoardSpeed.BindShip` self _output_get))

(event `self.ReceiveTick`
  (params (DeltaSeconds :type "Float (single-precision)"))
  (bind _raceend (`self.RaceEnd`))
  ;[1 1 1] TicK
  (set `self.Delta Seconds` DeltaSeconds)
  (if (`self.RaceStart`)
    (bind _output_get (set `self.NowSpeed` (`KismetMathLibrary.FInterpTo_Constant` (`self.NowSpeed`) (select `bool` _raceend :`false` (+ (* (`self.F_GetTargetSpeed`) 100.0) (`self.MinSpeed`))) (`self.Delta Seconds`) (select `bool` _raceend :`false` 100.0 :`true` 20.0))))
    (`SkeletalMeshComponent.SetPlayRate` (`self.SkeletalMesh1`) (`KismetMathLibrary.FClamp` (/ _output_get 200.0) 0.0 10.0))
    (set `MovementComponent.Velocity` (* (`SceneComponent.GetForwardVector` (`self.Arrow`)) (`self.NowSpeed`)) (`self.ProjectileMovement`))))

(event `Event_RaceEnd`
  ;[1 1 1] 结束游戏
  (set `self.RaceEnd` true))

(event `Event_GetSpeedUP`
  (params (BuffCount :type Integer))
  ;[1 1 1] 执行加速效果
  (for _ (range BuffCount)
    (`KismetArrayLibrary.Array_Add` (`self.TimeSticks`) (`KismetSystemLibrary.GetGameTimeInSeconds`))))

(fn `F_GetTargetSpeed`
  (returns (OutBuffCount :type Integer))
  (locals (CacheTimeStick :type "Array of Float (double-precision)") (DeletTImerStick :type "Array of Float (double-precision)"))
  (bind _output_get (set `local.CacheTimeStick` (`self.TimeSticks`)))
  (for _array_element _output_get
    (if (<= (+ _array_element (`self.SpeedTime`)) (`KismetSystemLibrary.GetGameTimeInSeconds`))
      (`KismetArrayLibrary.Array_Add` (`local.DeletTImerStick`) _array_element)))
  (for _array_element_2 (`local.DeletTImerStick`)
    (if (`KismetArrayLibrary.Array_Contains` (`self.TimeSticks`) _array_element_2)
      (`KismetArrayLibrary.Array_Remove` (`self.TimeSticks`) (`KismetArrayLibrary.Array_Find` (`self.TimeSticks`) _array_element_2))))
  (return (`KismetArrayLibrary.Array_Length` (`self.TimeSticks`))))

(fn `UserConstructionScript`)